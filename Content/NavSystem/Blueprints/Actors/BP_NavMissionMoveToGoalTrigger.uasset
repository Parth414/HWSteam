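; BP_NavMissionMoveToGoalTrigger is a move-to-goal mission trigger for the navigation system that removes itself when the player pawn overlaps it.
; Its Destroyed event calls Start on the BPC_NavElement component of NextMoveToGoalTrigger, if both are valid, so triggers chain into a sequence of goals.
; The hand-off hangs on destruction rather than overlap, so destroying the trigger by other means also starts the next element.
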(event `self.ReceiveActorBeginOverlap`
  (params (OtherActor :type "Actor Object Reference"))
  ;[1 1 1] OverlapEvents - Destroy self
  (if (== OtherActor (`GameplayStatics.GetPlayerPawn` 0))
    (`self.K2_DestroyActor`)))

(event `self.ReceiveDestroyed`
  (bind _returnvalue (`self.GetComponentByClass` (`self.NextMoveToGoalTrigger`) "/Game/NavSystem/Blueprints/Components/BPC_NavElement.BPC_NavElement_C"))
  (`/Engine/EditorBlueprintResources/StandardMacros.IsValid` (`self.NextMoveToGoalTrigger`)
    (:`Is Valid`
      (`/Engine/EditorBlueprintResources/StandardMacros.IsValid` _returnvalue
        (:`Is Valid`
          (`/Game/NavSystem/Blueprints/Components/BPC_NavElement.Start` _returnvalue))))))

(fn `UserConstructionScript`)