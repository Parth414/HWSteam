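; BP_NavEnemy is an enemy that wanders near its spawn location and is destroyed when its health runs out.
; BeginPlay stores the spawn location and starts a self-repeating AI MoveTo loop, which picks a new target on success or failure.
; Targets add random positive X and Y offsets up to WanderRadius, so wandering covers a square to one side of spawn.
; AnyDamage subtracts from Hp.
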(event `self.ReceiveBeginPlay`
  ;[1 1 1] Start Move Patrol
  (set `self.SpawnLoc` (`self.K2_GetActorLocation`))
  (`self.Start_AIMoveTo`))

(event `Start_AIMoveTo`
  ;[1 1 1] MoveTo Destination
  (bind _output_get (set `self.TargetLoc` (`KismetMathLibrary.MakeVector` (+ (`KismetMathLibrary.RandomFloatInRange` 0.0 (`self.WanderRadius`)) (.x (`self.SpawnLoc`))) (+ (`KismetMathLibrary.RandomFloatInRange` 0.0 (`self.WanderRadius`)) (.y (`self.SpawnLoc`))) (.z (`self.SpawnLoc`)))))
  (`|AIMoveTo` self _output_get null 15.0
    (:`OnSuccess`
      _)
    (:`OnFail`
      _))
  (`self.Start_AIMoveTo`))

(event `self.ReceiveAnyDamage`
  (params (Damage :type "Float (single-precision)") (DamageType :type "DamageType Object Reference") (InstigatedBy :type "Controller Object Reference") (DamageCauser :type "Actor Object Reference"))
  ;[1 1 1] Damage Events
  ;;[1 1 1] Subtract damage from health
  (bind _output_get (set `self.Hp` (- (`self.Hp`) Damage)))
  (if (<= _output_get 0.0)
    (`self.K2_DestroyActor`)))

(fn `UserConstructionScript`)