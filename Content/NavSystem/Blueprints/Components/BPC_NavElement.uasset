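; Actor component that makes its owner a navigation element with compass, indicator, enemy indicator, minimap, big map and radar icons.
; On BeginPlay, unless the owner is hidden, it registers with the player pawn's BPC_NavSystem; ReInit accepts another system, and EndPlay unregisters.
; It holds the icon widget references to toggle visibility or detach them together.
; Helpers provide the offset indicator location and a min/max distance check.
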(event `self.ReceiveBeginPlay`
  (if (not (`Actor.bHidden` (`self.GetOwner`)))
    (`self.Start`)))

(event `Start`
  (bind _returnvalue (`GameplayStatics.GetPlayerPawn` 0))
  (bind _returnvalue_2 (`Actor.GetComponentByClass` _returnvalue "/Game/NavSystem/Blueprints/Components/BPC_NavSystem.BPC_NavSystem_C"))
  (if (not (`self.IsInit`))
    (`/Engine/EditorBlueprintResources/StandardMacros.IsValid` _returnvalue
      (:`Is Valid`
        (`/Engine/EditorBlueprintResources/StandardMacros.IsValid` _returnvalue_2
          (:`Is Valid`
            (bind _output_get (set `self.NavSystem` _returnvalue_2))
            (`/Game/NavSystem/Blueprints/Components/BPC_NavSystem.ReqAddElement` _output_get self)
            (set `self.IsInit` true)))))))

(event `Init`
  (if (not (`Actor.bHidden` (`self.GetOwner`)))
    (`self.Start`)))

(event `ReInit`
  (params (InNavSystem :type "/Game/NavSystem/Blueprints/Components/BPC_NavSystem Object Reference"))
  (set `self.NavSystem` InNavSystem)
  (if (or (not (`Actor.bHidden` (`self.GetOwner`))) (`self.IsInit`))
    (`/Game/NavSystem/Blueprints/Components/BPC_NavSystem.ReqAddElement` (`self.NavSystem`) self)))

(event `SetCompassIconWidget`
  (params (CompassMarkWidget :type "UserWidget Object Reference"))
  (set `self.CompassIconWidgetRef` CompassMarkWidget))

(event `self.ReceiveEndPlay`
  (params (EndPlayReason :type "EEndPlayReason Enum" :default "Destroyed"))
  (`/Engine/EditorBlueprintResources/StandardMacros.IsValid` (`self.NavSystem`)
    (:`Is Valid`
      (`/Game/NavSystem/Blueprints/Components/BPC_NavSystem.RemoveElement` (`self.NavSystem`) self))))

(fn `CheckDistance`
  (params (Distance :type "Float (double-precision)"))
  (returns (ReturnValue :type Boolean))
  (return (and (>= Distance (`self.MinDistance`)) (<= Distance (`self.MaxDistance`)))))

(fn `GetOwnerIndicatorLoc`
  (returns (ReturnValue :type "Vector Structure"))
  (return (+ (`Actor.K2_GetActorLocation` (`self.GetOwner`)) (`self.IndicatorWorldOffset`))))

(fn `RemoveWidgetFromParent`
  (bind _indicatoriconwidgetref (`self.IndicatorIconWidgetRef`))
  (bind _compassiconwidgetref (`self.CompassIconWidgetRef`))
  (bind _radariconwidgetref (`self.RadarIconWidgetRef`))
  (bind _enemyindicatoriconwidgetref (`self.EnemyIndicatorIconWidgetRef`))
  (bind _minimapiconwidgetref (`self.MinimapIconWidgetRef`))
  (bind _bigmapiconwidgetref (`self.BigmapIconWidgetRef`))
  (`|ExecutionSequence`
    (:`then_0`
      (`/Engine/EditorBlueprintResources/StandardMacros.IsValid` _compassiconwidgetref
        (:`Is Valid`
          (`Widget.RemoveFromParent` _compassiconwidgetref))))
    (:`then_1`
      (`/Engine/EditorBlueprintResources/StandardMacros.IsValid` _indicatoriconwidgetref
        (:`Is Valid`
          (`Widget.RemoveFromParent` _indicatoriconwidgetref))))
    (:`then_2`
      (`/Engine/EditorBlueprintResources/StandardMacros.IsValid` _minimapiconwidgetref
        (:`Is Valid`
          (`Widget.RemoveFromParent` _minimapiconwidgetref))))
    (:`then_3`
      (`/Engine/EditorBlueprintResources/StandardMacros.IsValid` _bigmapiconwidgetref
        (:`Is Valid`
          (`Widget.RemoveFromParent` _bigmapiconwidgetref))))
    (:`then_4`
      (`/Engine/EditorBlueprintResources/StandardMacros.IsValid` _radariconwidgetref
        (:`Is Valid`
          (`Widget.RemoveFromParent` _radariconwidgetref))))
    (:`then_5`
      (`/Engine/EditorBlueprintResources/StandardMacros.IsValid` _enemyindicatoriconwidgetref
        (:`Is Valid`
          (`Widget.RemoveFromParent` _enemyindicatoriconwidgetref))))))

(fn `Show`
  (params (IsVisible :type Boolean))
  (locals (LocalIsVisible :type Boolean))
  (`/Engine/EditorBlueprintResources/StandardMacros.IsValid` (`self.NavSystem`)
    (:`Is Valid`
      (set `self.IsVisible` IsVisible)
      (set `local.LocalIsVisible` IsVisible)
      (`self.ShowUserWidget` (`self.CompassIconWidgetRef`) (`local.LocalIsVisible`))
      (`self.ShowUserWidget` (`self.IndicatorIconWidgetRef`) (`local.LocalIsVisible`))
      (`self.ShowUserWidget` (`self.EnemyIndicatorIconWidgetRef`) (`local.LocalIsVisible`))
      (`self.ShowUserWidget` (`self.MinimapIconWidgetRef`) (`local.LocalIsVisible`))
      (`self.ShowUserWidget` (`self.BigmapIconWidgetRef`) (`local.LocalIsVisible`))
      (`self.ShowUserWidget` (`self.RadarIconWidgetRef`) (`local.LocalIsVisible`)))))

(fn `ShowUserWidget`
  (params (UserWidget :type "UserWidget Object Reference") (IsShow :type Boolean))
  (locals (LocalUserWidget :type "UserWidget Object Reference"))
  (bind _localuserwidget (`local.LocalUserWidget`))
  (bind _output_get (set `local.LocalUserWidget` UserWidget))
  (`/Engine/EditorBlueprintResources/StandardMacros.IsValid` _output_get
    (:`Is Valid`
      (if IsShow
        (`Widget.SetVisibility` _localuserwidget "Visible")
        (else
          (`Widget.SetVisibility` _localuserwidget "Hidden"))))))

(fn `Use`
  (params (IsUse :type Boolean))
  (locals (LocalIsVisible :type Boolean))
  (set `self.IsUse` IsUse))