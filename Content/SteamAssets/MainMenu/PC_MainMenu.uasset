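; Main menu player controller that sets up the local player's identity at startup, using Steam when available.
; After a short delay, BeginPlay saves the unique net ID into PlayerInfo through a Game Instance message, or without Steam only sets PlayerName from a stored variable.
; Disconnected, never-executed chains would fetch the player's Steam avatar and forward friends marked Away, with avatars, to the Game Instance.
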(event `self.ReceiveBeginPlay`
  (`KismetSystemLibrary.Delay` 0.2)
  (if (`AdvancedSessionsLibrary.HasOnlineSubsystem` "STEAM")
    (bind _structout (setmembers `/Game/SteamAssets/S_PlayerInfo` :`StructRef` (`self.PlayerInfo`) :`SteamInfo` (`AdvancedSessionsLibrary.GetUniqueNetID` self)))
    (message `/Game/SteamAssets/BPI_GameInstance.SavePlayerInfo` (`GameplayStatics.GetGameInstance`) _structout)
    (else
      (set `self.PlayerName` (`KismetTextLibrary.Conv_StringToText` (`AdvancedSessionsLibrary.GetPlayerName` self))))))

(fn `GetPlayerName`
  (returns (PlayerName :type Text))
  (return (`KismetTextLibrary.Conv_StringToText` (`self.PlayerNameold`))))

(fn `UserConstructionScript`)