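; Main menu player controller that shows the menu at BeginPlay with UI-only input and handles multiplayer sessions.
; Events open host, options, loading and server browser widgets, reusing cached instances for all but the browser.
; LaunchLobby creates a session with the given player count and LAN flag, then opens Lobby as a listen server or shows an error widget on failure.
; Other events join or destroy sessions.
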(event `self.ReceiveBeginPlay`
  (`self.MainMenu` ; Has The Menu Already Been Drawn
    (:`then`
      _)
    (:`else`
      (bind _returnvalue (`|CreateWidget` "/Game/_Main/UI/W_MainMenu.W_MainMenu_C"))
      (bind _output_get (set `self.MainMenu` _returnvalue))))
  (`UserWidget.AddToViewport` _output_get 0)
  (set `self.bShowMouseCursor` true)
  (`WidgetBlueprintLibrary.SetInputMode_UIOnlyEx` self (`self.MainMenu`)))

(event `self.ShowHostMenu`
  (`self.HostMenu`
    (:`then`
      _)
    (:`else`
      (bind _returnvalue (`|CreateWidget` "/Game/_Main/UI/W_HostMenu.W_HostMenu_C"))
      (bind _output_get (set `self.HostMenu` _returnvalue))))
  (`UserWidget.AddToViewport` _output_get 0))

(event `self.ShowOptionsMenu`
  (`self.OptionsMenu`
    (:`then`
      _)
    (:`else`
      (bind _returnvalue (`|CreateWidget` "/Game/_Main/UI/W_OptionMenu.W_OptionMenu_C"))
      (bind _output_get (set `self.OptionsMenu` _returnvalue))))
  (`UserWidget.AddToViewport` _output_get 0))

(event `self.ShowServerMenu`
  (bind _returnvalue (`|CreateWidget` "/Game/_Main/UI/UI_ServerBrowser.UI_ServerBrowser_C"))
  (`UserWidget.AddToViewport` _returnvalue 0))

(event `self.ShowLoadingScreen`
  (`self.LoadingScreen`
    (:`then`
      _)
    (:`else`
      (bind _returnvalue (`|CreateWidget` "/Game/_Main/UI/W_LoadingScreen.W_LoadingScreen_C"))
      (bind _output_get (set `self.LoadingScreen` _returnvalue))))
  (`UserWidget.AddToViewport` _output_get 0))

(event `self.LaunchLobby`
  (params (NumberOfPlayers :type Integer) (`EnableLan?` :type Boolean) (ServerName :type Text))
  (bind _output_get (set `self.MaxPlayers` NumberOfPlayers))
  (set `self.ServerName` ServerName)
  (`self.ShowLoadingScreen`)
  (`CreateSessionCallbackProxy.CreateSession` (`GameplayStatics.GetPlayerController` 0) _output_get `EnableLan?`
    (:`OnSuccess`
      (`GameplayStatics.OpenLevel` "Lobby" true "listen"))
    (:`OnFailure`
      (bind _errorwindow (`self.ErrorWindow`)
        (:`then`
          (if (`Widget.IsInViewport` _errorwindow)
            (`Widget.RemoveFromParent` _errorwindow)
            (bind _returnvalue (`|CreateWidget` "/Game/_Main/UI/W_ErrorWidget.W_ErrorWidget_C" :!label _label))
            (bind _output_get_2 (set `self.ErrorWindow` _returnvalue))
            (`UserWidget.AddToViewport` _output_get_2 0)))
        (:`else`
          (goto _label))))))

(event `self.JoinServer`
  (params (SessionToJoin :type "BlueprintSessionResult Structure"))
  (`self.ShowLoadingScreen`)
  (`JoinSessionCallbackProxy.JoinSession` (`GameplayStatics.GetPlayerController` 0) SessionToJoin))

(event `self.DestroySessionCaller`
  (`DestroySessionCallbackProxy.DestroySession` null))

(fn `UserConstructionScript`)