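; BP_BaseCharacter_Child is a player character child Blueprint that adds keyboard control over the MovementLayer state.
; Holding Left Shift, C or X sets MovementLayer to a different enum value, and releasing any of them returns it to the first value.
; Keys are bound directly as key events, with the last press or release winning.
; The file only sets the state; BeginPlay, overlap and Tick are disabled stubs, and construction defers to the parent.
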(event `Key|LeftShift`
  (params (Key :type "Key Structure"))
  (:`Pressed`
    (set `self.MovementLayer` "NewEnumerator1"))
  (:`Released`
    (set `self.MovementLayer` "NewEnumerator0")))

(event `Key|C`
  (params (Key :type "Key Structure"))
  (:`Pressed`
    (set `self.MovementLayer` "NewEnumerator2"))
  (:`Released`
    (set `self.MovementLayer` "NewEnumerator0")))

(event `Key|X`
  (params (Key :type "Key Structure"))
  (:`Pressed`
    (set `self.MovementLayer` "NewEnumerator3"))
  (:`Released`
    (set `self.MovementLayer` "NewEnumerator0")))

(fn `UserConstructionScript`
  (`parent.UserConstructionScript`))